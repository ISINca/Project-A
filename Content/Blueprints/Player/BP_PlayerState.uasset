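; Player state Blueprint that tracks a player's team, current mission and kill, death and assist counts.
; Binds to mission start and end events, storing the mission data on start and setting a two-second timer, apparently to delay HUD creation.
; The HUD setup creates mission and tab-menu widgets using the team's mission state.
; Mission end prints win or loss, resets mission variables and removes the widgets.
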(event Custom|MissionStart_Event
  (params (MyTeam :type E_Team%20Enum :default "NewEnumerator2") (Mission :type BP%20Base%20Mission%20Object%20Reference))
  ;[1 1 1] Start Mission
  (Variables|Default|SetTeam MyTeam)
  (Variables|Default|SetCurrentMission Mission)
  (Variables|Default|SetOnMission? true)
  (Utilities|Time|SetTimerbyEvent (EventDispatchers|CreateEvent :!event Custom|AddHUDMission) 2.0))

(event Custom|MissionEnd_Event
  (params (TeamWinner :type E_Team%20Enum :default "NewEnumerator2"))
  ;[1 1 1] End Mission
  (CallFunction|WhoWin TeamWinner)
  (CallFunction|ResetMissionVariables)
  (CallFunction|RemoveHUDMission))

(event Custom|RemoveHUDMission
  ;[1 1 1] HUD Mission
  (Widget|RemovefromParent (Variables|Default|GetMissionHUD))
  (Widget|RemovefromParent (Variables|Default|GetTabmenuHUD)))

(event Custom|AddHUDMission
  (bind _currentmission (Variables|Default|GetCurrentMission))
  ;[1 1 1] HUD Mission
  (bind _returnvalue (UserInterface|CreateWidget "/Game/UI/HUD/W_MissionHUD.W_MissionHUD_C" (.AsBP%20Player%20Controller (Utilities|Casting|CastToBP_PlayerController (Components|GetOwner))) (Variables|Default|GetCurrentMission)))
  (bind _output_get (Variables|Default|SetMissionHUD _returnvalue))
  (UserInterface|Viewport|AddtoViewport _output_get 0)
  (Default|CallMissionStart(ForWidget) self (Utilities|Select :Index (Variables|Default|GetTeam) :NewEnumerator2 0 :NewEnumerator0 (Variables|/Game/Blueprints/Game/BP_BaseMission.BP_BaseMission_C|GetTeamA_State _currentmission) :NewEnumerator1 (Variables|/Game/Blueprints/Game/BP_BaseMission.BP_BaseMission_C|GetTeamB_State _currentmission)))
  (bind _returnvalue_2 (UserInterface|CreateWidget "/Game/UI/HUD/W_Tabmenu.W_Tabmenu_C" (.AsBP%20Player%20Controller (Utilities|Casting|CastToBP_PlayerController (Components|GetOwner))) (Variables|Default|GetCurrentMission)))
  (Variables|Default|SetTabmenuHUD _returnvalue_2))

(event Custom|AssinVaribles
  (bind _returnvalue (Components|GetOwner))
  (bind _asbp_player_controller (Utilities|Casting|CastToBP_PlayerController _returnvalue))
  ;[1 1 1] Assine Variables
  (Variables|Default|SetBP_PlayerController _asbp_player_controller)
  (Variables|Default|SetBP_PlayerCharacter (Variables|/Game/Blueprints/Player/BP_PlayerController.BP_PlayerController_C|GetPlayerCharacter _asbp_player_controller)))

(event EventBeginPlay
  ;[1 1 1] Begin play
  (EventDispatchers|BindEventtoMissionStart (EventDispatchers|CreateEvent :!event Custom|MissionStart_Event))
  (EventDispatchers|BindEventtoMissionEnd (EventDispatchers|CreateEvent :!event Custom|MissionEnd_Event)))

(event EventTick
  (params (DeltaSeconds :type Float%20%28single-precision%29)))

(fn ConstructionScript)

(fn AddDeath
  (Math|Integer|IncrementInt (Variables|KDA|GetDeaths)))

(fn AddKill
  (Math|Integer|IncrementInt (Variables|KDA|GetKills)))

(fn AddAssist
  (Math|Integer|IncrementInt (Variables|KDA|GetAssists)))

(fn GetDeaths
  (return (Variables|KDA|GetDeaths)))

(fn GetKills
  (return (Variables|KDA|GetKills)))

(fn GetAssists
  (return (Variables|KDA|GetAssists)))

(fn WhoWin
  (params (TeamWin :type E_Team%20Enum :default "NewEnumerator2"))
  (if (Utilities|Enum|Equal(Enum) TeamWin (Variables|Default|GetTeam))
    (Development|PrintString "You team win!")
    (elif (Utilities|Enum|Equal(Enum) TeamWin "NewEnumerator2")
      (Development|PrintString "All Players Blunder!")
      (else
        (Development|PrintString "You team lose!")))))

(fn ResetMissionVariables
  (Variables|Default|SetTeam "NewEnumerator2")
  (Variables|Default|SetCurrentMission 0)
  (Variables|Default|SetOnMission? false))