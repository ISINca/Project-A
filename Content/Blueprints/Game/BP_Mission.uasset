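; BP_Mission is a round-based mission Blueprint, currently a skeleton that mainly tracks elapsed round time.
; On BeginPlay it prints a debug start message and starts a looping one-second timer, whose RoundTimeTick adds a second to TimeCurrentRound and prints it.
; StartMission selects the first entry in Rounds but is not called here, while StopMission and ChangeRound are empty stubs.
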(event Custom|StartTimer
  (bind _returnvalue (Utilities|Time|SetTimerbyFunctionName 0 "RoundTimeTick" 1.0 true))
  (Variables|MissionState|SetRoundTimeTimer _returnvalue))

(event EventBeginPlay
  (Development|PrintString (Utilities|String|Append "Mission " (Utilities|GetDisplayName self) " starting") true true "(R=1.000000,G=0.384947,B=0.000000,A=1.000000)" 5.0)
  (CallFunction|StartTimer))

(fn ConstructionScript)

(fn StartMission
  (Variables|MissionRules|SetCurrentRound (Utilities|Array|Get(acopy) (Variables|MissionRules|GetRounds))))

(fn StopMission)

(fn ChangeRound)

(fn RoundTimeTick
  (bind _output_get (Variables|MissionState|SetTimeCurrentRound (+ (Variables|MissionState|GetTimeCurrentRound) (Math|Timespan|MakeTimespan 0 0 0 1))))
  (Development|PrintString (Utilities|String|ToString(Text) (Class|KismetTextLibrary|AsTimespanTimespan _output_get)) true true "(R=0.000000,G=0.660000,B=1.000000,A=1.000000)" 1.0))