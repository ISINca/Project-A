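; Base game mode that handles character death, spectating, player spawning and match start.
; On death it broadcasts the event, possesses the victim's controller into a spectator (following the instigator if valid, otherwise free), and starts the controller's respawn timer when auto-respawn is on.
; SpawnPlayer destroys any current pawn and spawns the character at a random free BP_GamePlayerSpawn.
; StartMatch broadcasts the match-started event.
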(fn ConstructionScript)

(fn CharacterDead
  (params (DeadCharacter :type BP%20Player%20Character%20Object%20Reference) (DeathInstigatior :type BP%20Player%20Controller%20Object%20Reference) (DeathFrom :type Actor%20Object%20Reference))
  (Default|CallCharDead DeadCharacter DeathInstigatior DeathFrom)
  (bind _asbp_player_controller (Utilities|Casting|CastToBP_PlayerController (Pawn|GetController DeadCharacter)))
  (CallFunction|SpawnSpectator _asbp_player_controller DeathInstigatior)
  (if (Variables|Default|GetAutoRespawn)
    (Default|LaunchRespawnTimer _asbp_player_controller (Variables|Default|GetRespawnTime))))

(fn SpawnPlayer
  (params (Player :type BP%20Player%20Controller%20Object%20Reference))
  (bind _returnvalue (Pawn|GetControlledPawn Player))
  (Utilities|IsValid _returnvalue
    (:Is%20Valid
      (Actor|DestroyActor _returnvalue))
    (:Is%20Not%20Valid
      _))
  (bind _freespawn (CallFunction|GetFreeSpawn))
  (bind _output_get (LocalVariables|SetLPlayerSpawn (Utilities|Array|Get(acopy) _freespawn (Math|Random|RandomInteger (Utilities|Array|LastIndex _freespawn)))))
  (Default|SpawnCharacter _output_get Player))

(fn GetFreeSpawn
  (bind _outactors (Actor|GetAllActorsOfClass "/Game/Blueprints/Game/BP_GamePlayerSpawn.BP_GamePlayerSpawn_C"))
  (for _array_element _outactors
    (if (Default|IsFree _array_element)
      (Utilities|Array|Add (LocalVariables|GetL_FreePoints) _array_element)))
  (return (LocalVariables|GetL_FreePoints)))

(fn SpawnSpectator
  (params (Player :type BP%20Player%20Controller%20Object%20Reference) (DeadInstigator :type BP%20Player%20Controller%20Object%20Reference))
  (bind _returnvalue (Utilities|IsValid DeadInstigator))
  (bind _returnvalue_2 (Pawn|GetControlledPawn DeadInstigator))
  (bind _returnvalue_3 (Game|SpawnActorfromClass (select _returnvalue "/Game/Blueprints/Player/BP_GameSpectator_CharFollow.BP_GameSpectator_CharFollow_C" "/Game/Blueprints/Player/BP_GameSpectator_Free.BP_GameSpectator_Free_C") (Transformation|GetActorTransform (select _returnvalue _returnvalue_2 (Pawn|GetControlledPawn Player))) "Undefined" Player 0))
  (bind _asbp_game_spectator_char_follow (Utilities|Casting|CastToBP_GameSpectator_CharFollow _returnvalue_3)
    (:then
      (Variables|/Game/Blueprints/Player/BP_GameSpectator_CharFollow.BP_GameSpectator_CharFollow_C|SetFollowCharacter _asbp_game_spectator_char_follow (.AsBP%20Player%20Character (Utilities|Casting|CastToBP_PlayerCharacter _returnvalue_2))))
    (:CastFailed
      _))
  (Pawn|Possess Player _returnvalue_3)
  (return _returnvalue_3))

(fn StartMatch
  (Default|CallMatchStarted))