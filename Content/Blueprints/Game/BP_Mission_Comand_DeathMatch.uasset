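; Team deathmatch mission Blueprint that scores kills for two teams and decides the match winner.
; UpdateDeathPoints runs the parent logic, then gives the killer's team a point via its PlayerState team.
; When a team reaches the point limit, it ends the mission.
; WhoWin compares both scores and sends the end-mission result for Team A, Team B, or no team on a tie.
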(fn UpdateDeathPoints
  (params (WhoDead :type BP%20Player%20Character%20Object%20Reference) (WhoKilled :type BP%20Player%20Controller%20Object%20Reference) (WhoAssist :type Map%20of%20BP%20Player%20Controller%20Object%20References%20to%20Float%20%28single-precision%29s))
  (|CallParentFunction WhoDead WhoKilled WhoAssist)
  (switch Utilities|FlowControl|Switch|SwitchonE_Team (Variables|/Game/Blueprints/Player/BP_PlayerState.BP_PlayerState_C|GetTeam (.AsBP%20Player%20State (Utilities|Casting|CastToBP_PlayerState (Variables|/Script/Engine.Controller|GetPlayerState WhoKilled))))
    (:NewEnumerator0
      (bind _result (Math|Integer|IncrementInt (Variables|Default|GetPointsTeamA))
        (:%20%20
          (bind _output_get (Variables|Default|SetPointsTeamA _result))
          (if (>= _output_get (Variables|Default|GetTeamPointsLimit))
            (CallFunction|EndMission)))))
    (:NewEnumerator1
      (bind _result_2 (Math|Integer|IncrementInt (Variables|Default|GetPointsTeamB))
        (:%20%20
          (bind _output_get_2 (Variables|Default|SetPointsTeamB _result_2))
          (if (>= _output_get_2 (Variables|Default|GetTeamPointsLimit))
            (CallFunction|EndMission)))))))

(fn WhoWin
  (if (> (Variables|Default|GetPointsTeamA) (Variables|Default|GetPointsTeamB))
    (CallFunction|SendDEndMissiontoTeam "NewEnumerator0")
    (elif (> (Variables|Default|GetPointsTeamB) (Variables|Default|GetPointsTeamA))
      (CallFunction|SendDEndMissiontoTeam "NewEnumerator1")
      (else
        (CallFunction|SendDEndMissiontoTeam "NewEnumerator2")))))