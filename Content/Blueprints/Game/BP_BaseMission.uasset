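; Base mission component that runs a timed team round from BeginPlay and handles character deaths during it.
; SetRounds adds a hardcoded test kill-the-other-team round, and a one-second timer counts it down; the kill limit is never checked.
; Deaths update kill, death and assist stats, spawn a spectator and optionally schedule a respawn.
; At time-out, it sends a fixed winner value to both teams' player states, then destroys itself.
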(event Custom|SetRounds
  (bind _rounds (Variables|MissionRules|GetRounds))
  ;[1 1 1] Test Set Round
  (bind _returnvalue (Utilities|Array|Add _rounds (Utilities|Struct|MakeS_RoundRules 1 "NewEnumerator1" "Kill all Team B!" "Kill all Team A!" 60 true 5 true)))
  (Variables|MissionRules|SetCurrentRound (Utilities|Array|Get(acopy) _rounds _returnvalue)))

(event Custom|StartMission
  ;[1 1 1] Start Mission
  (Development|PrintString (Utilities|String|Append "Mission " (Utilities|GetDisplayName self) " starting") true true "(R=1.000000,G=0.384947,B=0.000000,A=1.000000)" 5.0)
  (CallFunction|SetRounds)
  (CallFunction|StartRoundTimer)
  (Utilities|Time|SetTimerbyEvent (delegate Custom|CustomEvent_1) 1.0))

(event Custom|CharacterDeadOnMission
  (params (WhoDead :type BP%20Player%20Character%20Object%20Reference) (WhoKilled :type BP%20Player%20Controller%20Object%20Reference) (WhatKilled :type Actor%20Object%20Reference) (WhoAssist :type Map%20of%20BP%20Player%20Controller%20Object%20References%20to%20Float%20%28single-precision%29s))
  ;[1 1 1] What do when dead character, how play on mission
  (CallFunction|UpdateDeathPoints WhoDead WhoKilled WhoAssist)
  (Development|PrintString "Character dead on mission")
  (bind _spectator (Default|SpawnSpectator (.AsBP%20Base%20Gamemode (Utilities|Casting|CastToBP_BaseGamemode (Game|GetGameMode))) WhoDead WhoKilled))
  (if (Variables|MissionRules|Respawn|GetAutoRespawn)
    (Utilities|Time|SetTimerbyFunctionName (Pawn|GetController _spectator) "RespawnCharacter" (Variables|MissionRules|Respawn|GetRespawnTime))))

(event Custom|EndMission
  ;[1 1 1] Mission End
  (Development|PrintString (Utilities|String|Append "Mission " (Utilities|GetDisplayName self) " Ending") true true "(R=1.000000,G=0.384947,B=0.000000,A=1.000000)" 5.0)
  (CallFunction|WhoWin)
  (Utilities|FlowControl|Delay 5.0)
  (Components|DestroyComponent))

(event Custom|CustomEvent_1
  (for _array_element (Variables|Team|GetTeamA)
    (Utilities|Array|Add (Variables|Team|GetTeamA_State) (Variables|/Game/Blueprints/Player/BP_PlayerController.BP_PlayerController_C|GetBP_PlayerState _array_element)))
  (for _array_element_2 (Variables|Team|GetTeamB)
    (Utilities|Array|Add (Variables|Team|GetTeamB_State) (Variables|/Game/Blueprints/Player/BP_PlayerController.BP_PlayerController_C|GetBP_PlayerState _array_element_2))))

(event EventBeginPlay
  ;[1 1 1] BeginPlay
  (CallFunction|StartMission))

(fn RoundTimeTick
  (bind _output_get (Variables|MissionStates|SetTimeCurrentRound (- (Variables|MissionStates|GetTimeCurrentRound) (Math|Timespan|MakeTimespan 0 0 0 1))))
  (Utilities|FlowControl|Sequence
    (:then_1
      (if (== _output_get (Math|Timespan|MakeTimespan 0))
        (Utilities|Time|ClearandInvalidateTimerbyHandle (Variables|MissionStates|GetRoundTimerTimer))
        (CallFunction|EndMission)))))

(fn StartRoundTimer
  (Variables|MissionStates|SetTimeCurrentRound (Math|Timespan|MakeTimespan 0 0 0 (Utilities|Struct|BreakS_RoundRules (Variables|MissionRules|GetCurrentRound))))
  (bind _returnvalue (Utilities|Time|SetTimerbyFunctionName 0 "RoundTimeTick" 1.0 true))
  (Variables|MissionStates|SetRoundTimerTimer _returnvalue))

(fn UpdateDeathPoints
  (params (WhoDead :type BP%20Player%20Character%20Object%20Reference) (WhoKilled :type BP%20Player%20Controller%20Object%20Reference) (WhoAssist :type Map%20of%20BP%20Player%20Controller%20Object%20References%20to%20Float%20%28single-precision%29s))
  (Default|AddDeath (Variables|/Game/Blueprints/Player/BP_PlayerController.BP_PlayerController_C|GetBP_PlayerState (.AsBP%20Player%20Controller (Utilities|Casting|CastToBP_PlayerController (Pawn|GetController WhoDead)))))
  (Default|AddKill (Variables|/Game/Blueprints/Player/BP_PlayerController.BP_PlayerController_C|GetBP_PlayerState WhoKilled))
  (bind _keys (Utilities|Map|Keys WhoAssist))
  (for _array_element _keys
    (Default|AddAssist (Variables|/Game/Blueprints/Player/BP_PlayerController.BP_PlayerController_C|GetBP_PlayerState _array_element))))

(fn SendDEndMissiontoTeam
  (params (TeamWinner :type E_Team%20Enum :default "NewEnumerator2"))
  (Utilities|FlowControl|Sequence
    (:then_0
      (for _array_element (Variables|Team|GetTeamA_State)
        (Default|CallMissionEnd _array_element TeamWinner)))
    (:then_1
      (for _array_element_2 (Variables|Team|GetTeamB_State)
        (Default|CallMissionEnd _array_element_2 TeamWinner)))))

(fn WhoWin
  (CallFunction|SendDEndMissiontoTeam "NewEnumerator2"))