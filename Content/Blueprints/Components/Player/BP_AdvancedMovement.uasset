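; Player character component that adds parkour climbing, vaulting and sprinting.
; While Space is held, it repeats line traces every 0.1s during movement input to measure wall height, thickness and clearance, choosing climb, climb-over, get-up or vault.
; Moves disable collision, use Flying mode and play root-motion montages through SV_/MC_ events.
; Sprint has two speed paths; UpdateMoveSpeed's hard-coded branch always sets 300.
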(event Custom|SV_Set%20Component%20Collision
  (params (NewType :type ECollisionEnabled%20Enum :default "NoCollision"))
  (Collision|SetCollisionEnabled (Variables|/Script/Engine.Character|GetCapsuleComponent (Variables|Default|GetCharacter)) NewType))

(event Custom|SV_Movement%20Mode
  (params (NewMovementMode :type EMovementMode%20Enum :default "MOVE_None"))
  (Pawn|Components|CharacterMovement|SetMovementMode (Variables|/Script/Engine.Character|GetCharacterMovement (Variables|Default|GetCharacter)) NewMovementMode 0))

(event Custom|MC_PlayMontage
  (params (AnimMontage :type Anim%20Montage%20Object%20Reference) (InPlayRate :type Float%20%28single-precision%29) (StartSectionName :type Name))
  (Animation|PlayAnimMontage (Variables|Default|GetCharacter) AnimMontage InPlayRate "None"))

(event Custom|SprintPress1
  (params (PressDown :type Boolean))
  ;[1 1 1] Change Move Speed
  (Variables|Default|SetIsSprinting PressDown)
  (CallFunction|SVUpdateMoveSpeed))

(event Custom|ServerSprint
  (params (On :type Boolean))
  (if On
    (CallFunction|StartSprint)
    (else
      (CallFunction|StopSprint))))

(event Custom|SV_UpdateMoveSpeed
  ;[1 1 1] Change Move Speed
  (CallFunction|MCUpdateMoveSpeed))

(event Custom|MC_UpdateMoveSpeed
  ;[1 1 1] Change Move Speed
  (CallFunction|UpdateMoveSpeed))

(event Custom|SprintPress2
  (params (On :type Boolean))
  (CallFunction|ServerSprint On)
  (if On
    (CallFunction|StartSprint)
    (else
      (CallFunction|StopSprint))))

(event Custom|SV_SetActorLoc
  (params (NewLocation :type Vector))
  (Transformation|SetActorLocation (Variables|Default|GetCharacter) NewLocation false false))

(event Custom|Spacebar1
  (params (Spacebardown :type Boolean) (X :type Float%20%28single-precision%29) (Y :type Float%20%28single-precision%29))
  (bind _character (Variables|Default|GetCharacter))
  (bind _character_2 (Variables|Default|GetCharacter))
  (bind _character_3 (Variables|Default|GetCharacter))
  (bind _character_4 (Variables|Default|GetCharacter))
  (bind _returnvalue (Transformation|GetActorLocation _character))
  (bind _returnvalue_2 (Transformation|GetActorRotation _character_2))
  (bind _returnvalue_3 (Transformation|GetActorLocation _character_2))
  (bind _returnvalue_4 (Transformation|GetActorLocation _character_3))
  (bind _returnvalue_5 (Transformation|GetActorLocation _character_3))
  (bind _returnvalue_6 (Transformation|GetActorRotation _character_4))
  (bind _returnvalue_7 (Transformation|GetActorLocation _character_4))
  (bind _returnvalue_8 (- _returnvalue "0, 0,44.000000"))
  (bind _returnvalue_9 (+ _returnvalue_5 "0, 0,200.000000"))
  ;[1 1 1] Basic Logic for Spacebar
  (if Spacebardown
    (Variables|Default|SetSpacePress true)
    (Utilities|FlowControl|Sequence :!label _label
      (:then_0
        (if (not (and (== X 0.0) (== Y 0.0)))
          (if (not (Variables|Default|GetIsClimbing))
            ;[1 1 1] Check for wall
            (bind (_outhit _returnvalue_10) (Collision|LineTraceForObjects _returnvalue_8 (+ _returnvalue_8 (* (Transformation|GetActorForwardVector _character) (Variables|Default|GetFarCheck))) (Utilities|Array|MakeArray "ObjectTypeQuery1") true 0 "ForDuration"))
            (if _returnvalue_10
              (Variables|Default|SetWallLocation (.Location (Collision|BreakHitResult _outhit)))
              (Variables|Default|SetWallNormal (.Normal (Collision|BreakHitResult _outhit)))
              ;[1 1 1] Check for Height
              (bind (_outhit_2 _returnvalue_11) (Collision|LineTraceForObjects (+ (+ (* (Math|Vector|GetForwardVector (Math|Rotator|MakeRotfromX (Variables|Default|GetWallNormal))) -1e+01) (Variables|Default|GetWallLocation)) "0, 0,200.000000") (- (+ (+ (* (Math|Vector|GetForwardVector (Math|Rotator|MakeRotfromX (Variables|Default|GetWallNormal))) -1e+01) (Variables|Default|GetWallLocation)) "0, 0,200.000000") "0, 0,200.000000") (Utilities|Array|MakeArray "ObjectTypeQuery1") true 0 "ForDuration"))
              (if _returnvalue_11
                (Variables|Default|SetWallHeight (.Location (Collision|BreakHitResult _outhit_2)))
                ;[1 1 1] Check for Obsticles in-front
                (bind _returnvalue_12 (Collision|LineTraceForObjects (+ (Variables|Default|GetWallHeight) "0, 0,1.000000") (+ (Variables|Default|GetWallHeight) "30.000000, 0,1.000000") (Utilities|Array|MakeArray "ObjectTypeQuery1") false 0 "ForDuration"))
                (if (not _returnvalue_12)
                  (Utilities|FlowControl|Sequence
                    (:then_0
                      ;[1 1 1] Climb/Vault logic
                      (if (> (.Z (Math|Vector|BreakVector (- (Variables|Default|GetWallHeight) (Variables|Default|GetWallLocation)))) 6e+01)
                        (Variables|Default|SetShouldClimb true)
                        (else
                          (Variables|Default|SetShouldClimb false))))
                    (:then_1
                      ;[1 1 1] Check for Wall Thiccness
                      (bind (_outhit_3 _returnvalue_13) (Collision|LineTraceForObjects (+ (+ (* (Math|Vector|GetForwardVector (Math|Rotator|MakeRotfromX (Variables|Default|GetWallNormal))) -5e+01) (Variables|Default|GetWallLocation)) "0, 0,250.000000") (- (+ (+ (* (Math|Vector|GetForwardVector (Math|Rotator|MakeRotfromX (Variables|Default|GetWallNormal))) -5e+01) (Variables|Default|GetWallLocation)) "0, 0,250.000000") "0, 0,300.000000") (Utilities|Array|MakeArray "ObjectTypeQuery1") true 0 "ForDuration"))
                      (if _returnvalue_13
                        (Variables|Default|SetOtherWallHeight (.Location (Collision|BreakHitResult _outhit_3)))
                        (Utilities|FlowControl|Sequence
                          (:then_0
                            ;[1 1 1] Get over the wall logic
                            (if (> (.Z (Math|Vector|BreakVector (- (Variables|Default|GetWallHeight) (Variables|Default|GetOtherWallHeight)))) 3e+01)
                              (Variables|Default|SetIsWallThick false)
                              (else
                                (Variables|Default|SetIsWallThick true))))
                          (:then_1
                            (if (Variables|Default|GetShouldClimb) :!label _label_2
                              (Development|PrintString "Climb")
                              (Utilities|FlowControl|Sequence
                                (:then_0
                                  ;[1 1 1] Check for obscticles over head
                                  (bind _returnvalue_14 (Collision|LineTraceForObjects _returnvalue_9 (+ _returnvalue_9 (* (Transformation|GetActorForwardVector _character_3) 7e+01)) (Utilities|Array|MakeArray "ObjectTypeQuery1") true 0 "ForDuration"))
                                  (if _returnvalue_14
                                    (Variables|Default|SetCanClimb false))
                                  (bind _returnvalue_15 (Collision|LineTraceForObjects _returnvalue_4 (+ _returnvalue_4 "0, 0,200.000000") (Utilities|Array|MakeArray "ObjectTypeQuery1") true 0 "ForDuration"))
                                  (if _returnvalue_15
                                    (Variables|Default|SetCanClimb false)))
                                (:then_1
                                  (if (Variables|Default|GetCanClimb)
                                    (Variables|Default|SetIsClimbing true)
                                    ;[1 1 1] Climbing/Get over the wall
                                    (CallFunction|SVSetComponentCollision "NoCollision")
                                    (CallFunction|SVMovementMode "MOVE_Flying")
                                    (CallFunction|SVSetActorRot (Math|Rotator|MakeRotator (.roll _returnvalue_2) (.pitch _returnvalue_2) (+ (.Yaw (Math|Rotator|BreakRotator (Math|Rotator|MakeRotfromX (Variables|Default|GetWallNormal)))) 1.8e+02)))
                                    (CallFunction|SVSetActorLoc (+ (* (Math|Vector|GetForwardVector (Math|Rotator|MakeRotfromX (Variables|Default|GetWallNormal))) -1.0) (Transformation|GetActorLocation _character_2)))
                                    (CallFunction|SVSetActorLoc (Math|Vector|MakeVector (.x _returnvalue_3) (.y _returnvalue_3) (- (.Z (Math|Vector|BreakVector (Variables|Default|GetWallHeight))) 44.0)))
                                    (CallFunction|SVPlayMontage "/Game/Assets/Characters/ParkourAnimations/MQ_Climb_RM_Montage.MQ_Climb_RM_Montage" 1.0 "None")
                                    (Utilities|FlowControl|Delay 0.8)
                                    (if (Variables|Default|GetIsWallThick)
                                      (CallFunction|SVSetComponentCollision "QueryAndPhysics")
                                      (CallFunction|SVMovementMode "MOVE_Walking")
                                      (else
                                        (CallFunction|SVPlayMontage "/Game/Assets/Characters/ParkourAnimations/MQ_JumpingDownFromWall_RM_Montage.MQ_JumpingDownFromWall_RM_Montage" 1.0 "None")
                                        (Utilities|FlowControl|Delay 1.0)
                                        (CallFunction|SVSetComponentCollision "QueryAndPhysics")
                                        (CallFunction|SVMovementMode "MOVE_Falling")))
                                    (Variables|Default|SetIsClimbing false))))
                              (else
                                (Development|PrintString "Vault")
                                (Variables|Default|SetIsClimbing true)
                                ;[1 1 1] GetUp/Vault
                                (CallFunction|SVSetComponentCollision "NoCollision")
                                (CallFunction|SVMovementMode "MOVE_Flying")
                                (CallFunction|SVSetActorRot (Math|Rotator|MakeRotator (.roll _returnvalue_6) (.pitch _returnvalue_6) (+ (.Yaw (Math|Rotator|BreakRotator (Math|Rotator|MakeRotfromX (Variables|Default|GetWallNormal)))) 1.8e+02)))
                                (if (Variables|Default|GetIsWallThick)
                                  (CallFunction|SVSetActorLoc (+ (* (Math|Vector|GetForwardVector (Math|Rotator|MakeRotfromX (Variables|Default|GetWallNormal))) 3e+01) (Transformation|GetActorLocation _character_4)))
                                  (CallFunction|SVPlayMontage "/Game/Assets/Characters/ParkourAnimations/MQ_GettingUp_RM_Montage.MQ_GettingUp_RM_Montage" 1.0 "None")
                                  (Utilities|FlowControl|Delay 0.8)
                                  (else
                                    (CallFunction|SVSetActorLoc (Math|Vector|MakeVector (.x _returnvalue_7) (.y _returnvalue_7) (- (.Z (Math|Vector|BreakVector (Variables|Default|GetWallHeight))) (Variables|Default|GetVaultHate))))
                                    (CallFunction|SVPlayMontage "/Game/Assets/Characters/ParkourAnimations/MQ_Vault_RM_Montage.MQ_Vault_RM_Montage" 1.0 "None")
                                    (Utilities|FlowControl|Delay 0.9)))
                                (CallFunction|SVSetComponentCollision "QueryAndPhysics")
                                (CallFunction|SVMovementMode "MOVE_Walking")
                                (Variables|Default|SetIsClimbing false)))))
                        (else
                          (Variables|Default|SetIsWallThick false)
                          (goto _label_2)))))))))))
      (:then_1
        (Utilities|FlowControl|Delay 0.1)
        (if (Variables|Default|GetSpacePress)
          (goto _label))))
    (else
      (Variables|Default|SetSpacePress false))))

(event Custom|SV_SetActorRot
  (params (NewRotation :type Rotator))
  (Transformation|SetActorRotation (Variables|Default|GetCharacter) NewRotation))

(event Custom|SV_PlayMontage
  (params (AnimMontage :type Anim%20Montage%20Object%20Reference) (InPlayRate :type Float%20%28single-precision%29) (StartSectionName :type Name))
  (CallFunction|MCPlayMontage AnimMontage InPlayRate "None"))

(event EventBeginPlay
  ;[1 1 1] Set Character
  (bind _asbp_player_character (Utilities|Casting|CastToBP_PlayerCharacter (Components|GetOwner)))
  (bind _output_get (Variables|Default|SetCharacter _asbp_player_character))
  (Variables|Default|SetDefaultSpeed (Variables|/Script/Engine.CharacterMovementComponent|GetMaxWalkSpeed (Variables|/Script/Engine.Character|GetCharacterMovement _output_get))))

(fn StartSprint
  (if (CallFunction|CanSprint)
    (Variables|/Script/Engine.CharacterMovementComponent|SetMaxWalkSpeed (Variables|/Script/Engine.Character|GetCharacterMovement (Variables|Default|GetCharacter)) (Variables|Default|GetSprintSpeed))))

(fn StopSprint
  (Variables|/Script/Engine.CharacterMovementComponent|SetMaxWalkSpeed (Variables|/Script/Engine.Character|GetCharacterMovement (Variables|Default|GetCharacter)) (Variables|Default|GetWalkSpeed)))

(fn UpdateMoveSpeed
  (bind _character (Variables|Default|GetCharacter))
  (bind _charactermovement (Variables|/Script/Engine.Character|GetCharacterMovement _character))
  (if true
    (Variables|/Script/Engine.CharacterMovementComponent|SetMaxWalkSpeed _charactermovement 3e+02)
    (elif (Variables|Default|GetIsSprinting)
      (Variables|/Script/Engine.CharacterMovementComponent|SetMaxWalkSpeed _charactermovement 6e+02)
      (else
        (Variables|/Script/Engine.CharacterMovementComponent|SetMaxWalkSpeed _charactermovement 4.5e+02)))))

(fn CanSprint
  (return true))