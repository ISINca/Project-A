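; Firearm weapon Blueprint that handles hitscan firing, distance-based damage and ammo reloading.
; UseWeapon gates on the parent, traces from the follow camera, re-traces from the character's eyes to that point, then applies point damage.
; Damage falls linearly from DropoffRange to MinDamageRange; beyond that it returns zero because the MinDamage branch's comparison is inverted.
; Reloading is authority-only and timer-delayed, auto-triggering on an empty magazine; debug traces and messages remain.
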(event Custom|DEBUG_DrawServerTrace
  (params (Start :type Vector) (End :type Vector) (Hit :type Vector))
  (Rendering|Debug|DrawDebugLine Start End "(R=0.885417,G=0.467433,B=0.000000,A=1.000000)" 5.0 2.0)
  (Rendering|Debug|DrawDebugSphere Hit 2e+01 6 "(R=1.000000,G=0.007579,B=0.000000,A=1.000000)" 5.0 2.0))

(fn ConstructionScript
  (|CallParentFunction))

(fn GetFireTrace
  (bind _asbp_player_character (Utilities|Casting|CastToBP_PlayerCharacter (Game|GetInstigator)))
  (bind _desiredview (Class|CameraComponent|GetCameraView (Variables|/Game/Blueprints/Player/BP_PlayerCharacter.BP_PlayerCharacter_C|GetFollowCamera _asbp_player_character) 0.0))
  (bind _outhit (Class|KismetSystemLibrary|CapsuleTraceSingleforObjects (.Location (Utilities|Struct|BreakMinimalViewInfo _desiredview)) (+ (.Location (Utilities|Struct|BreakMinimalViewInfo _desiredview)) (* (Math|Vector|Normalize (Math|Rotator|GetRotationXVector (.Rotation (Utilities|Struct|BreakMinimalViewInfo _desiredview)))) (Variables|Default|GetMaxRange))) 0.0 0.0 (Utilities|Array|MakeArray "ObjectTypeQuery1" "ObjectTypeQuery2" "ObjectTypeQuery3") false 0 "None" true))
  (bind _outhit_2 (Collision|LineTraceForObjects (.OutLocation (Actor|GetActorEyesViewPoint _asbp_player_character)) (.Location (Collision|BreakHitResult _outhit)) (Utilities|Array|MakeArray "ObjectTypeQuery1" "ObjectTypeQuery2" "ObjectTypeQuery3") false (Utilities|Array|MakeArray self (Game|GetInstigator)) "None"))
  (CallFunction|DEBUGDrawServerTrace (.TraceStart (Collision|BreakHitResult _outhit_2)) (.TraceEnd (Collision|BreakHitResult _outhit_2)) (.Location (Collision|BreakHitResult _outhit_2)))
  (return _outhit_2))

(fn UseWeapon
  (bind _used (|CallParentFunction))
  (CallFunction|PrintMessageDebug (Utilities|String|Append (Utilities|String|ToString(Integer) (Variables|Default|GetCurrentAmmo)) "|" (Utilities|String|ToString(Integer) (Variables|Default|GetTotalAmmo))) "(R=0.000000,G=0.082951,B=0.635417,A=1.000000)" 1.0 false)
  (if _used
    (bind _hit (CallFunction|GetFireTrace))
    (bind _currantdamage (CallFunction|DamageCalculator (.Distance (Collision|BreakHitResult _hit))))
    (Game|Damage|ApplyPointDamage (.HitActor (Collision|BreakHitResult _hit)) _currantdamage (Math|Vector|GetUnitDirection(Vector) (.TraceEnd (Collision|BreakHitResult _hit)) (.TraceStart (Collision|BreakHitResult _hit))) _hit (Game|GetInstigatorController) self)
    (return true)
    (else
      (if (Math|Boolean|ANDBoolean (<= (Variables|Default|GetCurrentAmmo) 0) (> (Variables|Default|GetTotalAmmo) 0) (not (Variables|Default|GetFireActive self)))
        (CallFunction|ReloadWeapon))
      (return false))))

(fn ReloadWeapon
  (Networking|SwitchHasAuthority
    (:Authority
      (if (Math|Boolean|ANDBoolean (!= (Utilities|GetClassDefaults (Utilities|GetClass self)) (Variables|Default|GetCurrentAmmo)) (> (Variables|Default|GetTotalAmmo) 0) (not (Variables|Reload|GetReloading)))
        (Variables|Reload|SetReloading true)
        (CallFunction|PrintMessageDebug "Reloading" "(R=0.000000,G=0.639191,B=0.994792,A=1.000000)" 2.0 false)
        (Utilities|Time|SetTimerbyFunctionName 0 "ReloadWeaponEnd" (Variables|Reload|GetReloadTime))
        (else
          (CallFunction|PrintMessageDebug "Not able to reload" "(R=0.000000,G=0.639191,B=0.994792,A=1.000000)" 2.0 true))))))

(fn ReloadWeaponEnd
  (LocalVariables|SetAmmoToReload (Math|Integer|Min(Integer) (- (Utilities|GetClassDefaults (Utilities|GetClass self)) (Variables|Default|GetCurrentAmmo)) (Variables|Default|GetTotalAmmo)))
  (Variables|Default|SetCurrentAmmo (+ (Variables|Default|GetCurrentAmmo) (LocalVariables|GetAmmoToReload)))
  (Variables|Default|SetTotalAmmo (- (Variables|Default|GetTotalAmmo) (LocalVariables|GetAmmoToReload)))
  (Variables|Reload|SetReloading false)
  (CallFunction|PrintMessageDebug (Utilities|String|Append (Utilities|String|ToString(Integer) (Variables|Default|GetCurrentAmmo)) "|" (Utilities|String|ToString(Integer) (Variables|Default|GetTotalAmmo))) "(R=0.000000,G=0.082951,B=0.635417,A=1.000000)" 1.0 false))

(fn DamageCalculator
  (params (Distance :type Float%20%28single-precision%29))
  (if (<= Distance (Variables|Default|GetDropoffRange))
    (return (Variables|Default|GetDamage))
    (elif (and (>= (Variables|Default|GetMinDamageRange) Distance) (> Distance (Variables|Default|GetDropoffRange)))
      (return (|((MinDam-(MinDamRange*((MaxDam-MinDam)/(Doff-MinDamRange))))+(Dist*((MaxDam-MinDam)/(Doff-MinDamRange)))) (Variables|Default|GetDamage) (Variables|Default|GetMinDamage) (Variables|Default|GetDropoffRange) Distance (Variables|Default|GetMinDamageRange)))
      (elif (and (> (Variables|Default|GetMinDamageRange) Distance) (< Distance (Variables|Default|GetMaxRange)))
        (return (Variables|Default|GetMinDamage))
        (else
          (return 0.0))))))