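; Grenade weapon projectile that explodes on a timer, dealing full radial damage without falloff.
; On BeginPlay, the authority launches the physics capsule forward with a random spin impulse and starts the fuse timer.
; When the fuse ends, Explode applies the damage, credited to the instigator's controller, and destroys the actor.
; Destruction triggers the explosion particle effect only on non-authority machines, reusing a rocket launcher emitter.
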(event EventBeginPlay
  (Networking|SwitchHasAuthority
    (:Authority
      (Physics|AddImpulse (Variables|Default|GetCapsule) (* (Transformation|GetActorForwardVector) 1e+03) "None" false)
      (Class|PrimitiveComponent|AddAngularImpulseinRadians (Variables|Default|GetCapsule) (Math|Vector|MakeVector (Math|Random|RandomFloatinRange -5e+02 5e+02) (Math|Random|RandomFloatinRange -5e+02 5e+02) (Math|Random|RandomFloatinRange -5e+02 5e+02)) "None" false)
      (Utilities|Time|SetTimerbyFunctionName 0 "Explode" (Variables|Default|GetExplodeTimer)))))

(event EventDestroyed
  (|CallParentFunction)
  (Networking|SwitchHasAuthority
    (:Remote
      (Effects|SpawnEmitteratLocation "/Game/Assets/MilitaryWeapSilver/FX/P_RocketLauncher_Explosion_01.P_RocketLauncher_Explosion_01" (Transformation|GetActorLocation)))))

(fn ConstructionScript
  (|CallParentFunction))

(fn Explode
  (Game|Damage|ApplyRadialDamage (Variables|Default|GetDamage) (Transformation|GetActorLocation) (Variables|Default|GetDamageRadius) 0 0 self (Game|GetInstigatorController) true "ECC_Visibility")
  (Actor|DestroyActor))