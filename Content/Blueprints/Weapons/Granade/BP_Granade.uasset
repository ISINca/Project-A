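; BP_Granade is a grenade weapon that throws a grenade projectile when used.
; UseWeapon runs the parent logic and calls TrowGranade only if that succeeds.
; TrowGranade spawns BP_WeaponProjectile_Granage just ahead of a socket on the instigating player character's mesh, using the owner's rotation and passing on Damage and Instigator.
; It does nothing for instigators other than BP_PlayerCharacter, and HoldGranade is an empty stub.
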(event EventBeginPlay)

(event Collision|EventActorBeginOverlap
  (params (OtherActor :type Actor%20Object%20Reference)))

(event EventTick
  (params (DeltaSeconds :type Float%20%28single-precision%29)))

(fn ConstructionScript
  (|CallParentFunction))

(fn TrowGranade
  (bind _returnvalue (Components|GetOwner))
  (bind _asbp_player_character (Utilities|Casting|CastToBP_PlayerCharacter (Game|GetInstigator)))
  (Game|SpawnActorfromClass "/Game/Blueprints/Weapons/Granade/BP_WeaponProjectile_Granage.BP_WeaponProjectile_Granage_C" (Math|Transform|MakeTransform (+ (Transformation|GetSocketLocation (Variables|/Script/Engine.Character|GetMesh _asbp_player_character) (Variables|Default|GetDefaultSocketName)) (* (Transformation|GetActorForwardVector _returnvalue) 1e+01)) (Transformation|GetActorRotation _returnvalue)) "Undefined" 0 (Variables|Default|GetDamage) (Game|GetInstigator)))

(fn HoldGranade)

(fn UseWeapon
  (bind _used (|CallParentFunction))
  (if _used
    (CallFunction|TrowGranade))
  (return _used))