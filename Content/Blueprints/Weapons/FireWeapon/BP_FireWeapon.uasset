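; Firearm weapon Blueprint that handles hitscan shooting, spread, recoil and timed reloading.
; UseWeapon calls Shot, which traces from the camera with random spread, then from the muzzle to that hit, applying point damage with distance falloff.
; Projectile and impact emitters spawn only on the Remote authority branch, while reload runs only on Authority.
; Shots grow spread and add random controller kick; timers recover spread toward a modifiable minimum.
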(event Custom|AddRecoilServer
  (bind _characterowner (Variables|Default|GetCharacterOwner))
  ;[1 1 1] Recoil System (Simple system)
  (Pawn|Input|AddControllerPitchInput _characterowner (Math|Random|RandomFloatinRange -0.1 -0.5))
  (Pawn|Input|AddControllerYawInput _characterowner (Math|Random|RandomFloatinRange 0.2 -0.2)))

(event Custom|MuzzleFire
  (bind _meshweapon (Variables|Default|GetMeshWeapon))
  ;[1 1 1] Emitter/Fire trace
  (Networking|SwitchHasAuthority
    (:Authority
      _)
    (:Remote
      _))
  (Effects|SpawnEmitteratLocation (Variables|Fire|GetMuzzleFireEmitter) (Transformation|GetSocketLocation _meshweapon "MuzzleFlash") (Transformation|GetSocketRotation _meshweapon "MuzzleFlash")))

(event Custom|SpawnProjectile
  (params (Transform :type Transform))
  ;[1 1 1] Emitter/Fire trace
  (Networking|SwitchHasAuthority
    (:Remote
      (Game|SpawnActorfromClass (Variables|Default|GetProjectile) Transform "Undefined" 0 0))))

(event Custom|DEBUG_DrawServerTrace
  (params (HitTrace :type Hit%20Result%20Structure) (Color :type Linear%20Color%20Structure) (HitRadius :type Float%20%28single-precision%29))
  ;[1 0.02083 0.02083] Debug draw trace
)

(event Custom|SpawnEmitter
  ;[1 1 1] Emitter/Fire trace
  (Networking|SwitchHasAuthority
    (:Remote
      (Fire|MultySpawnEmitter (Variables|Default|GetHitInfo)))))

(fn ConstructionScript
  (bind _spreaddefault (Variables|Accuracy|GetSpreadDefault))
  (|CallParentFunction)
  (Variables|Accuracy|SetCurrentSpread _spreaddefault)
  (Variables|Accuracy|SetSpreadMin _spreaddefault))

(fn Shot
  (bind _array (Utilities|Array|MakeArray "ObjectTypeQuery1" "ObjectTypeQuery2" "ObjectTypeQuery3"))
  (bind _meshweapon (Variables|Default|GetMeshWeapon))
  (bind _returnvalue (Transformation|GetSocketLocation _meshweapon "MuzzleFlash"))
  (bind _asbp_player_character (Utilities|Casting|CastToBP_PlayerCharacter (Game|GetInstigator)))
  (bind (_start _end) (Fire|GetShotDirection))
  (bind _outhit (Collision|LineTraceForObjects _start _end _array false (Utilities|Array|MakeArray self _asbp_player_character) "None" :!pinned true)) ; First trace from camera to center screen
  (CallFunction|DEBUGDrawServerTrace _outhit "(R=0.916667,G=0.208228,B=0.180866,A=1.000000)" 1e+01)
  (LocalVariables|SetHitTrue (Math|Vector|NotEqual(Vector) (.Location (Collision|BreakHitResult _outhit)) "0, 0, 0" 0.0001))
  (bind _outhit_2 (Collision|LineTraceForObjects (Transformation|GetSocketLocation (Variables|Default|GetMeshWeapon) "MuzzleFlash") (+ (.Location (Collision|BreakHitResult _outhit)) (Math|Vector|GetForwardVector (Variables|/Game/Blueprints/Player/BP_PlayerCharacter.BP_PlayerCharacter_C|GetFollowCamera _asbp_player_character))) _array false (Utilities|Array|MakeArray self _asbp_player_character) "None" :!pinned true)) ; Second trace from Muzzle weapon to hit first trace
  (LocalVariables|SetHitResult2 _outhit_2)
  (CallFunction|SpawnProjectile (Math|Transform|MakeTransform _returnvalue (Math|Rotator|FindLookatRotation _returnvalue (Math|Vector|SelectVector (.TraceEnd (Collision|BreakHitResult (LocalVariables|GetHitResult2))) (.TraceEnd (Collision|BreakHitResult _outhit)) (LocalVariables|GetHitTrue)))))
  (CallFunction|DEBUGDrawServerTrace _outhit_2 "(R=0.000000,G=0.916667,B=0.133705,A=1.000000)" 15.0)
  (if true
    (Utilities|Array|SetArrayElem (Variables|Default|GetHitInfo) 0 (.Location (Collision|BreakHitResult (LocalVariables|GetHitResult2))) true)
    ;[1 1 1] Apply Damage
    (if (> (Fire|DamageCalculator (.Distance (Collision|BreakHitResult (LocalVariables|GetHitResult2)))) 0.0)
      (Game|Damage|ApplyPointDamage (.HitActor (Collision|BreakHitResult (LocalVariables|GetHitResult2))) (Fire|DamageCalculator (.Distance (Collision|BreakHitResult (LocalVariables|GetHitResult2)))) (Math|Vector|GetUnitDirection(Vector) (.TraceEnd (Collision|BreakHitResult (LocalVariables|GetHitResult2))) (.TraceStart (Collision|BreakHitResult (LocalVariables|GetHitResult2)))) (LocalVariables|GetHitResult2) (Game|GetInstigatorController) self))
    (return (.Location (Collision|BreakHitResult (LocalVariables|GetHitResult2))) true)
    (else
      (return "0, 0, 0" false))))

(fn UseWeapon
  (bind _used (|CallParentFunction))
  (if _used
    (bind _hit_ (Fire|Shot))
    (if _hit_
      (CallFunction|SpawnEmitter))
    (Accuracy|AddSpreadonFire)
    (CallFunction|AddRecoilServer)
    (CallFunction|MuzzleFire)
    (return true)
    (else
      (if (Math|Boolean|ANDBoolean (<= (Variables|Default|GetCurrentAmmo) 0) (> (Variables|Default|GetTotalAmmo) 0) (not (Variables|Default|GetFireActive self)))
        (Reload|ReloadWeapon))
      (return false))))

(fn ReloadWeapon
  (Networking|SwitchHasAuthority
    (:Authority
      (if (Math|Boolean|ANDBoolean (!= (.CurrentAmmo (Utilities|GetClassDefaults (Utilities|GetClass self))) (Variables|Default|GetCurrentAmmo)) (> (Variables|Default|GetTotalAmmo) 0) (not (Variables|Reload|GetReloading)))
        (Variables|Reload|SetReloading true)
        (CallFunction|PrintMessageDebug "Reloading" "(R=0.000000,G=0.639191,B=0.994792,A=1.000000)" 2.0 false)
        (Utilities|Time|SetTimerbyFunctionName 0 "ReloadWeaponEnd" (Variables|Reload|GetReloadTime))
        (else
          (CallFunction|PrintMessageDebug "Not able to reload" "(R=0.000000,G=0.639191,B=0.994792,A=1.000000)" 2.0 true))))))

(fn ReloadWeaponEnd
  (LocalVariables|SetAmmoToReload (Math|Integer|Min(Integer) (- (.CurrentAmmo (Utilities|GetClassDefaults (Utilities|GetClass self))) (Variables|Default|GetCurrentAmmo)) (Variables|Default|GetTotalAmmo)))
  (Variables|Default|SetCurrentAmmo (+ (Variables|Default|GetCurrentAmmo) (LocalVariables|GetAmmoToReload)))
  (Variables|Default|SetTotalAmmo (- (Variables|Default|GetTotalAmmo) (LocalVariables|GetAmmoToReload)))
  (Variables|Reload|SetReloading false)
  (CallFunction|PrintMessageDebug (Utilities|String|Append (Utilities|String|ToString(Integer) (Variables|Default|GetCurrentAmmo)) "|" (Utilities|String|ToString(Integer) (Variables|Default|GetTotalAmmo))) "(R=0.000000,G=0.082951,B=0.635417,A=1.000000)" 1.0 false))

(fn DamageCalculator
  (params (Distance :type Float%20%28single-precision%29))
  (if (<= Distance (Variables|Range|GetDropoffRange))
    (return (Variables|Default|GetDamage))
    (elif (and (>= (Variables|Range|GetMinDamageRange) Distance) (> Distance (Variables|Range|GetDropoffRange)))
      (return (/ (Math|Conversions|ToFloat(Integer) (Math|Float|Ceil (* 100 (|((MinDam-(MinDamRange*((MaxDam-MinDam)/(Doff-MinDamRange))))+(Dist*((MaxDam-MinDam)/(Doff-MinDamRange)))) (Variables|Default|GetDamage) (Variables|Range|GetMinDamage) (Variables|Range|GetDropoffRange) Distance (Variables|Range|GetMinDamageRange))))) 1e+02))
      (elif (and (>= (Variables|Range|GetMaxRange) Distance) (> Distance (Variables|Range|GetMinDamageRange)))
        (return (Variables|Range|GetMinDamage))
        (else
          (return 0.0))))))

(fn GetShotDirection
  (bind _currentspread (Variables|Accuracy|GetCurrentSpread))
  (bind _returnvalue (* _currentspread -1.0))
  (bind _asbp_player_character (Utilities|Casting|CastToBP_PlayerCharacter (Game|GetInstigator)))
  (return (Transformation|GetWorldLocation (Variables|/Game/Blueprints/Player/BP_PlayerCharacter.BP_PlayerCharacter_C|GetFollowCamera _asbp_player_character)) (+ (+ (Transformation|GetWorldLocation (Variables|/Game/Blueprints/Player/BP_PlayerCharacter.BP_PlayerCharacter_C|GetFollowCamera _asbp_player_character)) (* (Math|Vector|GetForwardVector (Variables|/Game/Blueprints/Player/BP_PlayerCharacter.BP_PlayerCharacter_C|GetFollowCamera _asbp_player_character)) (Variables|Range|GetMaxRange))) (Math|Vector|MakeVector (Math|Random|RandomFloatinRange _returnvalue _currentspread) (Math|Random|RandomFloatinRange _returnvalue _currentspread) (Math|Random|RandomFloatinRange _returnvalue _currentspread)))))

(fn MultySpawnEmitter
  (params (NewParam :type Array%20of%20Vectors))
  (for _index (range 0 (- (Utilities|Array|Length NewParam) 1))
    (Effects|SpawnEmitteratLocation "/Game/Assets/MilitaryWeapSilver/FX/P_Impact_Metal_Medium_01.P_Impact_Metal_Medium_01" (Utilities|Array|Get(acopy) NewParam _index) "0, 0, 0" "1.000000,1.000000,1.000000" true "AutoRelease")))

(fn AddSpreadonFire
  (Utilities|Time|ClearandInvalidateTimerbyHandle (Variables|Accuracy|Recovery|GetStartRecoveryTimer))
  (Variables|Accuracy|SetCurrentSpread (Math|Float|Min(Float) (* (Variables|Accuracy|GetCurrentSpread) (Variables|Accuracy|Mods|GetSpreadPerShot)) (Variables|Accuracy|GetSpreadMax)))
  (bind _returnvalue (Utilities|Time|SetTimerbyFunctionName 0 "StartSpreadRecovery" (Variables|Accuracy|Recovery|GetSpreadRecoveryDelay)))
  (Variables|Accuracy|Recovery|SetStartRecoveryTimer _returnvalue))

(fn SetReload
  (params (Reloading :type Boolean))
  (Variables|Reload|SetReloading Reloading))

(fn ChangeSpread
  (params (Mod :type Float%20%28single-precision%29) (On :type Boolean))
  (Utilities|Time|ClearandInvalidateTimerbyHandle (Variables|Accuracy|Recovery|GetStartRecoveryTimer))
  (if On
    (Variables|Accuracy|SetSpreadMin (Math|Float|Min(Float) (* (Variables|Accuracy|GetSpreadMin) Mod) (Variables|Accuracy|GetSpreadMax)))
    (else
      (bind _output_get (Variables|Accuracy|SetSpreadMin (Math|Float|Min(Float) (/ (Variables|Accuracy|GetSpreadMin) Mod) (Variables|Accuracy|GetSpreadMax))))
      (Variables|Accuracy|SetCurrentSpread (Math|Float|Max(Float) _output_get (Variables|Accuracy|GetCurrentSpread)))))
  (bind _returnvalue (Utilities|Time|SetTimerbyFunctionName 0 "StartSpreadRecovery" (Variables|Accuracy|Recovery|GetSpreadRecoveryDelay)))
  (Variables|Accuracy|Recovery|SetStartRecoveryTimer _returnvalue))

(fn GetSpread
  (return (Variables|Accuracy|GetCurrentSpread)))

(fn SetSpread
  (params (CurrentSpread :type Float%20%28single-precision%29))
  (Variables|Accuracy|SetCurrentSpread CurrentSpread))

(fn SpreadRecovery
  (if (and (not (== (Variables|Accuracy|GetCurrentSpread) (Variables|Accuracy|GetSpreadMin))) (not (Variables|Default|GetFireActive)))
    (bind _output_get (Variables|Accuracy|SetCurrentSpread (Math|Float|Max(Float) (- (Variables|Accuracy|GetCurrentSpread) (Variables|Accuracy|Recovery|GetSpreadRecoveryPerDelay)) (Variables|Accuracy|GetSpreadMin))))
    (else
      (Utilities|Time|ClearandInvalidateTimerbyHandle (Variables|Accuracy|Recovery|GetSpreadRecoveryTimer)))))

(fn StartSpreadRecovery
  (if (Variables|Accuracy|GetRecoverySpread)
    (bind _returnvalue (Utilities|Time|SetTimerbyFunctionName 0 "SpreadRecovery" (Variables|Accuracy|Recovery|GetSpreadRecoveryDelay) true))
    (Variables|Accuracy|Recovery|SetSpreadRecoveryTimer _returnvalue)))