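; BP_Weapon is a weapon Blueprint that handles ammo, fire rate and aim zoom for the player character.
; UseWeapon spends a round and starts an interval timer whose EndShot callback fires again in autofire mode until StopUseWeapon or empty ammo.
; For zoom type 1, a timeline narrows the owner's follow-camera FOV and shifts the camera forward, reversing on release.
; It spawns no projectile or trace itself.
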(event Custom|ZoomWeapon
  (params (Zoom :type Boolean))
  (bind _characterowner (Variables|Default|GetCharacterOwner))
  (bind _followcamera (Variables|/Game/Blueprints/Player/BP_PlayerCharacter.BP_PlayerCharacter_C|GetFollowCamera _characterowner))
  (switch int (Variables|Zoom|GetZoomType)
    (:1
      (if Zoom
        (bind _zooming (Timeline|Zoomline Play)
          (:Update
            (Variables|/Script/Engine.CameraComponent|SetFieldOfView _followcamera (- (Variables|Zoom|GetZoomDefault) (* _zooming (- (Variables|Zoom|GetZoomDefault) (Variables|Zoom|GetZoomValue)))))
            (Transformation|SetRelativeLocation _followcamera (Math|Vector|MakeVector (* _zooming 1e+02) 0.0 4e+01) false false)))
        (else
          (Timeline|Zoomline Reverse))))))

(fn ConstructionScript)

(fn StopUseWeapon
  (Variables|Fire|SetFireActive false))

(fn UseWeapon
  (if (and (not (Variables|Fire|GetFireIntervalActive)) (> (Variables|Ammo|GetCurrentAmmo) 0))
    (Math|Integer|DecrementInt (Variables|Ammo|GetCurrentAmmo)
      (:%20%20
        (Utilities|Time|SetTimerbyFunctionName 0 "EndShot" (Variables|Fire|GetFireInterval))
        (Variables|Fire|SetFireIntervalActive true)
        (if (== (Variables|Fire|GetCurrentFireMode) 0)
          (Variables|Fire|SetFireActive true))
        (return true)))
    (else
      (Variables|Fire|SetFireActive false)
      (return false))))

(fn EndShot
  (Variables|Fire|SetFireIntervalActive false)
  (if (and (== (Variables|Fire|GetCurrentFireMode) 0) (Variables|Fire|GetFireActive))
    (CallFunction|UseWeapon)))

(fn SetCharacterOwner
  (bind _asbp_player_character (Utilities|Casting|CastToBP_PlayerCharacter (Game|GetPlayerCharacter 0)))
  (bind _output_get (Variables|Default|SetCharacterOwner _asbp_player_character))
  (return _output_get))

(fn GetFireIntervalon
  (return (Variables|Fire|GetFireIntervalActive)))